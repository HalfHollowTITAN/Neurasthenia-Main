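; Wall-buy actor that sells the assault rifle to the player for points.
; Overlapping its text trigger shows an "E" key prompt with the cost on the character's HUD, and leaving hides it.
; UnlockAR checks the first player's points, then sets the rifle unlock, deducts the cost, plays a purchase sound, switches to that weapon and destroys the wall-buy.
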(event OnComponentBeginOverlap(TextTrigger)
  (params (OverlappedComponent :type Primitive%20Component%20Object%20Reference) (OtherActor :type Actor%20Object%20Reference) (OtherComp :type Primitive%20Component%20Object%20Reference) (OtherBodyIndex :type Integer) (bFromSweep :type Boolean) (SweepResult :type Hit%20Result%20Structure%20%28by%20ref%29))
  (bind _asfirst_person_character (Utilities|Casting|CastToFirstPersonCharacter OtherActor))
  (Default|ChangeKeyText(WallBuy) (Variables|/Game/Blueprints/Character/FirstPersonCharacter.FirstPersonCharacter_C|GetHUD _asfirst_person_character) "E " (Utilities|Text|ToText(Integer) (Variables|Default|GetCost))))

(event OnComponentEndOverlap(TextTrigger)
  (params (OverlappedComponent :type Primitive%20Component%20Object%20Reference) (OtherActor :type Actor%20Object%20Reference) (OtherComp :type Primitive%20Component%20Object%20Reference) (OtherBodyIndex :type Integer))
  (bind _asfirst_person_character (Utilities|Casting|CastToFirstPersonCharacter OtherActor))
  (Default|HideText (Variables|/Game/Blueprints/Character/FirstPersonCharacter.FirstPersonCharacter_C|GetHUD _asfirst_person_character)))

(event Custom|UnlockAR
  (bind _returnvalue (Game|GetPlayerCharacter 0))
  (bind _asfirst_person_character (Utilities|Casting|CastToFirstPersonCharacter _returnvalue))
  ;[1 1 1] if the player has enough points, the weapon's unlock bool will be set to tree and it will be equip along with the repective mag ammo
  (if (>= (Variables|/Game/Blueprints/Character/FirstPersonCharacter.FirstPersonCharacter_C|GetPoints _asfirst_person_character) (Variables|Default|GetCost))
    (Variables|/Game/Blueprints/Character/FirstPersonCharacter.FirstPersonCharacter_C|SetAssualtRifleUnlock _asfirst_person_character true)
    (Audio|PlaySoundatLocation "/Game/Sounds/PurchaseSound.PurchaseSound" (Variables|/Script/Engine.SceneComponent|GetRelativeLocation (Variables|Default|GetArrow)) "0, 0, 0" 1.0 1.0 0.0 0 0 0)
    (Variables|/Game/Blueprints/Character/FirstPersonCharacter.FirstPersonCharacter_C|SetPoints _asfirst_person_character (- (Variables|/Game/Blueprints/Character/FirstPersonCharacter.FirstPersonCharacter_C|GetPoints _asfirst_person_character) (Variables|Default|GetCost)))
    (Variables|/Game/Blueprints/Character/FirstPersonCharacter.FirstPersonCharacter_C|SetWeaponSelectionINT _asfirst_person_character 3)
    (Default|SwitchWeapon _asfirst_person_character)
    (Actor|DestroyActor)))

(fn ConstructionScript
  (|CallParentFunction))