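; Projectile Blueprint for a bullet that moves forward at constant speed and destroys itself when its lifetime runs out.
; Tick offsets it along its forward vector without sweep, so hits come from Box overlaps.
; Actors implementing BPI_AI_Damagable receive GunDamage and award points.
; Runner and Walker zombies also get ZombieDies called and destroy the bullet immediately; BulletHealth drops per hit but is never checked here.
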(event OnComponentBeginOverlap(Box)
  (params (OverlappedComponent :type Primitive%20Component%20Object%20Reference) (OtherActor :type Actor%20Object%20Reference) (OtherComp :type Primitive%20Component%20Object%20Reference) (OtherBodyIndex :type Integer) (bFromSweep :type Boolean) (SweepResult :type Hit%20Result%20Structure%20%28by%20ref%29))
  ;[1 1 1] Check to see if a damageable actor has been hit. If it has then the bullet's health will drop and it will deal damage. When the bullet has passed through 3 eneimes, it will despawn(Bullet Damages is set by the equip weapon)
  (bind _output_get (Variables|Default|SetOwningHitActor OtherActor))
  (if (Utilities|DoesObjectImplementInterface _output_get "/Game/AI/BPI_AI_Damagable.BPI_AI_Damagable_C")
    (Class|BPIAIDamagable|CustomDamageEvent(Message) (Variables|Default|GetOwningHitActor) (Variables|Default|GetGunDamage) 10)
    (Variables|Default|SetBulletHealth (- (Variables|Default|GetBulletHealth) 3e+01))
    (if (== (Utilities|GetClass (Variables|Default|GetOwningHitActor)) "/Game/AI/BP_ZombieAI_Runner.BP_ZombieAI_Runner_C")
      (bind _asbp_zombie_ai_runner (Utilities|Casting|CastToBP_ZombieAI_Runner (Variables|Default|GetOwningHitActor)))
      (Default|ZombieDies _asbp_zombie_ai_runner)
      (Actor|DestroyActor :!label _label)
      (elif (== (Utilities|GetClass (Variables|Default|GetOwningHitActor)) "/Game/AI/BP_ZombieAI_Walker.BP_ZombieAI_Walker_C")
        (bind _asbp_zombie_ai_walker (Utilities|Casting|CastToBP_ZombieAI_Walker (Variables|Default|GetOwningHitActor)))
        (Default|ZombieDies _asbp_zombie_ai_walker)
        (goto _label)))))

(event EventTick
  (params (DeltaSeconds :type Float%20%28single-precision%29))
  ;[1 1 1] Bullet Movement
  ;;[0.1289 0.2903 1] Bullet will travel forward at a constant rate when spawned
  (Transformation|AddActorWorldOffset (* (Transformation|GetActorForwardVector) (* DeltaSeconds (Variables|Default|GetMoveSpeed))))
  (if (>= (Utilities|Time|GetRealTimeSeconds) (+ (Variables|Default|GetStartTime) (Variables|Default|GetLifetime)))
    (Actor|DestroyActor)))

(event EventBeginPlay
  ;[1 1 1] Bullet Movement
  (Variables|Default|SetStartTime (Utilities|Time|GetRealTimeSeconds))
  (bind _asfirst_person_character (Utilities|Casting|CastToFirstPersonCharacter (Game|GetPlayerCharacter 0)))
  (Variables|Default|SetAs%20First%20Person%20Character _asfirst_person_character))

(fn ConstructionScript)