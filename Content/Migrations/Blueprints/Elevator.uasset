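; Two-level elevator actor whose pad travels between top and bottom floors, with sliding doors and HUD interaction prompts.
; MovePad plays or reverses a movement timeline based on IsTopLevel, which overlap triggers at each end update, while IsMoving blocks re-triggering.
; On arrival, door timelines open that floor's door and close the other.
; Call and pad triggers show prompts to the player, with collision toggled to suit the pad's state.
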(event OnComponentBeginOverlap(PadInteraction)
  (params (OverlappedComponent :type Primitive%20Component%20Object%20Reference) (OtherActor :type Actor%20Object%20Reference) (OtherComp :type Primitive%20Component%20Object%20Reference) (OtherBodyIndex :type Integer) (bFromSweep :type Boolean) (SweepResult :type Hit%20Result%20Structure%20%28by%20ref%29))
  ;[1 1 1] When the player steps into a corresponding trigger, the interaction text will be printed based on which trigger they are standing on and will be removed when the player steps out of it
  ;;[0.3255 0.1098 1] Shows and hides the pad interaction text
  (bind _asfirst_person_character (Utilities|Casting|CastToFirstPersonCharacter OtherActor))
  (Default|ChangeKeyText(Elevator) (Variables|/Game/Blueprints/Character/FirstPersonCharacter.FirstPersonCharacter_C|GetHUD _asfirst_person_character) " to move floors"))

(event OnComponentBeginOverlap(PadIsTop)
  (params (OverlappedComponent :type Primitive%20Component%20Object%20Reference) (OtherActor :type Actor%20Object%20Reference) (OtherComp :type Primitive%20Component%20Object%20Reference) (OtherBodyIndex :type Integer) (bFromSweep :type Boolean) (SweepResult :type Hit%20Result%20Structure%20%28by%20ref%29))
  ;[1 1 1] Pad location functionality
  (if (== OtherComp (Variables|Default|GetPad))
    (Variables|Default|SetIsTopLevel true)))

(event OnComponentEndOverlap(PadInteraction)
  (params (OverlappedComponent :type Primitive%20Component%20Object%20Reference) (OtherActor :type Actor%20Object%20Reference) (OtherComp :type Primitive%20Component%20Object%20Reference) (OtherBodyIndex :type Integer))
  ;[1 1 1] When the player steps into a corresponding trigger, the interaction text will be printed based on which trigger they are standing on and will be removed when the player steps out of it
  ;;[0.3255 0.1098 1] Shows and hides the pad interaction text
  (bind _asfirst_person_character (Utilities|Casting|CastToFirstPersonCharacter OtherActor))
  (Default|HideText (Variables|/Game/Blueprints/Character/FirstPersonCharacter.FirstPersonCharacter_C|GetHUD _asfirst_person_character)))

(event OnComponentBeginOverlap(CallTopTrigger)
  (params (OverlappedComponent :type Primitive%20Component%20Object%20Reference) (OtherActor :type Actor%20Object%20Reference) (OtherComp :type Primitive%20Component%20Object%20Reference) (OtherBodyIndex :type Integer) (bFromSweep :type Boolean) (SweepResult :type Hit%20Result%20Structure%20%28by%20ref%29))
  ;[1 1 1] When the player steps into a corresponding trigger, the interaction text will be printed based on which trigger they are standing on and will be removed when the player steps out of it
  ;;[0.3255 0.1098 1] Shows and hides the Top Calling interaction text
  (bind _asfirst_person_character (Utilities|Casting|CastToFirstPersonCharacter OtherActor))
  (Default|ChangeKeyText(Elevator) (Variables|/Game/Blueprints/Character/FirstPersonCharacter.FirstPersonCharacter_C|GetHUD _asfirst_person_character) " to call the elevator"))

(event OnComponentBeginOverlap(PadIsBottom)
  (params (OverlappedComponent :type Primitive%20Component%20Object%20Reference) (OtherActor :type Actor%20Object%20Reference) (OtherComp :type Primitive%20Component%20Object%20Reference) (OtherBodyIndex :type Integer) (bFromSweep :type Boolean) (SweepResult :type Hit%20Result%20Structure%20%28by%20ref%29))
  ;[1 1 1] Pad location functionality
  (if (== OtherComp (Variables|Default|GetPad))
    (Variables|Default|SetIsTopLevel false)))

(event OnComponentBeginOverlap(CallBottomTrigger)
  (params (OverlappedComponent :type Primitive%20Component%20Object%20Reference) (OtherActor :type Actor%20Object%20Reference) (OtherComp :type Primitive%20Component%20Object%20Reference) (OtherBodyIndex :type Integer) (bFromSweep :type Boolean) (SweepResult :type Hit%20Result%20Structure%20%28by%20ref%29))
  ;[1 1 1] When the player steps into a corresponding trigger, the interaction text will be printed based on which trigger they are standing on and will be removed when the player steps out of it
  ;;[0.3255 0.1098 1] Shows and hides the Bottom Calling interaction text
  (bind _asfirst_person_character (Utilities|Casting|CastToFirstPersonCharacter OtherActor))
  (Default|ChangeKeyText(Elevator) (Variables|/Game/Blueprints/Character/FirstPersonCharacter.FirstPersonCharacter_C|GetHUD _asfirst_person_character) " to call the elevator"))

(event OnComponentEndOverlap(CallBottomTrigger)
  (params (OverlappedComponent :type Primitive%20Component%20Object%20Reference) (OtherActor :type Actor%20Object%20Reference) (OtherComp :type Primitive%20Component%20Object%20Reference) (OtherBodyIndex :type Integer))
  ;[1 1 1] When the player steps into a corresponding trigger, the interaction text will be printed based on which trigger they are standing on and will be removed when the player steps out of it
  ;;[0.3255 0.1098 1] Shows and hides the Bottom Calling interaction text
  (bind _asfirst_person_character (Utilities|Casting|CastToFirstPersonCharacter OtherActor))
  (Default|HideText (Variables|/Game/Blueprints/Character/FirstPersonCharacter.FirstPersonCharacter_C|GetHUD _asfirst_person_character)))

(event OnComponentEndOverlap(CallTopTrigger)
  (params (OverlappedComponent :type Primitive%20Component%20Object%20Reference) (OtherActor :type Actor%20Object%20Reference) (OtherComp :type Primitive%20Component%20Object%20Reference) (OtherBodyIndex :type Integer))
  ;[1 1 1] When the player steps into a corresponding trigger, the interaction text will be printed based on which trigger they are standing on and will be removed when the player steps out of it
  ;;[0.3255 0.1098 1] Shows and hides the Top Calling interaction text
  (bind _asfirst_person_character (Utilities|Casting|CastToFirstPersonCharacter OtherActor))
  (Default|HideText (Variables|/Game/Blueprints/Character/FirstPersonCharacter.FirstPersonCharacter_C|GetHUD _asfirst_person_character)))

(event Custom|Open%20Door
  ;[1 1 1] Opens the elevator doors based on where the pad is after it has landed and closes the corresponding door that is has travelled away from
  (if (not (Variables|Default|GetIsMoving))
    (if (Variables|Default|GetIsTopLevel)
      (Utilities|FlowControl|Sequence
        (:then_0
          (bind _moveup (Timeline|OpenTopDoor PlayFromStart)
            (:Update
              (Transformation|SetRelativeLocation (Variables|Default|GetTopDoor) (Math|Vector|Lerp(Vector) "109.455582, 0,292.983673" "109.455383, 0,422.152191" _moveup) false false))
            (:Finished
              (Collision|SetCollisionEnabled (Variables|Default|GetPadInteraction) "QueryOnly" :!label _label))))
        (:then_1
          (bind _moveup_2 (Timeline|OpenBottomDoor ReverseFromEnd)
            (:Update
              (Transformation|SetRelativeLocationAndRotation (Variables|Default|GetBottomDoor) (Math|Vector|Lerp(Vector) "109.456802, 0,-299.360535" "109.456802, 0,-169.906754" _moveup_2) "0, 0, 0" false false))
            (:Finished
              (goto _label)))))
      (else
        (Utilities|FlowControl|Sequence
          (:then_0
            (Timeline|OpenBottomDoor PlayFromStart))
          (:then_1
            (Timeline|OpenTopDoor ReverseFromEnd)))))))

(event Custom|MovePad
  ;[1 1 1] If the pad is not at the top it will move to the. If it is at the top the the animation will reverse and will move to the bottom
  (CallFunction|TextTriggerActivation)
  (if (not (Variables|Default|GetIsMoving))
    (Variables|Default|SetIsMoving true)
    (if (Variables|Default|GetIsTopLevel)
      (bind _bottom_top (Timeline|PadMovement PlayFromStart)
        (:Update
          (Transformation|SetRelativeLocation (Variables|Default|GetPad) (Math|Vector|Lerp(Vector) (Variables|Default|GetTopLevelVec) (Variables|Default|GetBottomLevelVec) _bottom_top) false false))
        (:Finished
          (Variables|Default|SetIsMoving false)
          (CallFunction|OpenDoor)))
      (else
        (Timeline|PadMovement ReverseFromEnd)))))

(event Custom|TextTriggerActivation
  ;[1 1 1] Turns the interaction text triggers on and off based on what level the pad is on
  (Utilities|HideText)
  (Utilities|FlowControl|Sequence
    (:then_0
      (if (Variables|Default|GetIsTopLevel)
        (Collision|SetCollisionEnabled (Variables|Default|GetCallTopTrigger) "QueryOnly")
        (Collision|SetCollisionEnabled (Variables|Default|GetCallBottomTrigger) "NoCollision")
        (else
          (Collision|SetCollisionEnabled (Variables|Default|GetCallTopTrigger) "NoCollision")
          (Collision|SetCollisionEnabled (Variables|Default|GetCallBottomTrigger) "QueryOnly"))))
    (:then_1
      (Utilities|HideText)
      (Collision|SetCollisionEnabled (Variables|Default|GetPadInteraction) "NoCollision"))))

(event EventBeginPlay
  ;[1 1 1] Pad location functionality
  (Variables|Default|SetIsTopLevel false))

(fn ConstructionScript)