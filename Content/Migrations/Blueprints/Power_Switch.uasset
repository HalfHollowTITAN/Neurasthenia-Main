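; Power switch actor that starts its linked lights off and, when PowerOn is called, powers up the level's lights and a door.
; BeginPlay zeroes each linked spotlight and swaps its mesh material.
; PowerOn animates the switch pivot by timeline, plays a sound, restores the lights and sets Powered.
; It also turns on all B_CourtyardLight actors from inside the light loop and moves only the first DoorRef entry, cast to B_PackADoor.
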(event Custom|PowerOn
  ;[1 1 1] Power on function. Will turn on all lights in the level and open any doors that require power to open.
  (Utilities|FlowControl|Sequence
    (:then_0
      (bind _newtrack_0 (Timeline|SwitchMoving PlayFromStart)
        (:Update
          (Transformation|SetRelativeRotation (Variables|Default|GetSwitchPivot) (Math|Rotator|MakeRotator _newtrack_0 0.0 0.0) false false))))
    (:then_1
      (Audio|PlaySoundatLocation "/Game/Sounds/WAVS/Barrier.Barrier" (Variables|Default|GetSoundVector) "0, 0, 0" 1.0 1.0 0.0 0 0 0))
    (:then_2
      (for _array_element (Variables|Default|GetLights)
        (Utilities|IsValid (Actor|GetComponentbyClass _array_element "/Script/Engine.SpotLightComponent")
          (:Is%20Valid
            (Rendering|Components|Light|SetIntensity (Actor|GetComponentbyClass _array_element "/Script/Engine.SpotLightComponent") 1e+02)
            (Rendering|Material|SetMaterial (Actor|GetComponentbyClass _array_element "/Script/Engine.StaticMeshComponent") 0 "/Game/Materials/Light.Light")
            (Variables|Default|SetPowered true)
            (bind _outactors (Actor|GetAllActorsOfClass "/Game/Blueprints/Blockout/B_CourtyardLight.B_CourtyardLight_C"))
            (for _array_element_2 _outactors
              (Default|TurnLightson _array_element_2))))))
    (:then_3
      (bind _asb_pack_adoor (Utilities|Casting|CastToB_PackADoor (Utilities|Array|Get(acopy) (Variables|Default|GetDoorRef))))
      (Default|MoveDoor _asb_pack_adoor))))

(event EventBeginPlay
  ;[1 1 1] Turns lights in array off from the start of level
  (for _array_element (Variables|Default|GetLights)
    (Utilities|IsValid (Actor|GetComponentbyClass _array_element "/Script/Engine.SpotLightComponent")
      (:Is%20Valid
        (Rendering|Components|Light|SetIntensity (Actor|GetComponentbyClass _array_element "/Script/Engine.SpotLightComponent") 0.0)
        (Rendering|Material|SetMaterial (Actor|GetComponentbyClass _array_element "/Script/Engine.StaticMeshComponent") 0 "/Game/Materials/M_light.M_light")))))

(fn ConstructionScript)