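; B_Metal_Door is a purchasable sliding double door that the player opens permanently by spending points.
; Entering or leaving its trigger shows or hides a HUD prompt with the cost.
; OpenDoor checks the player's points, deducts the cost, plays buzzer and purchase sounds, and slides both panels apart with a timeline lerp.
; It then destroys the trigger, removing the prompt.
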(event OnComponentBeginOverlap(Trigger)
  (params (OverlappedComponent :type Primitive%20Component%20Object%20Reference) (OtherActor :type Actor%20Object%20Reference) (OtherComp :type Primitive%20Component%20Object%20Reference) (OtherBodyIndex :type Integer) (bFromSweep :type Boolean) (SweepResult :type Hit%20Result%20Structure%20%28by%20ref%29))
  ;[1 1 1] When player walks into "Trigger", the cost text will be translated to match the variable
  (bind _asfirst_person_character (Utilities|Casting|CastToFirstPersonCharacter OtherActor))
  (Default|ChangeKeyText(Buy) (Variables|/Game/Blueprints/Character/FirstPersonCharacter.FirstPersonCharacter_C|GetHUD _asfirst_person_character) "E" (Utilities|Text|ToText(Integer) (Variables|Default|GetCost))))

(event OnComponentEndOverlap(Trigger)
  (params (OverlappedComponent :type Primitive%20Component%20Object%20Reference) (OtherActor :type Actor%20Object%20Reference) (OtherComp :type Primitive%20Component%20Object%20Reference) (OtherBodyIndex :type Integer))
  ;[1 1 1] When the player leaves the "Trigger", the text will be hidden
  (bind _asfirst_person_character (Utilities|Casting|CastToFirstPersonCharacter OtherActor))
  (Default|HideText (Variables|/Game/Blueprints/Character/FirstPersonCharacter.FirstPersonCharacter_C|GetHUD _asfirst_person_character)))

(event Custom|OpenDoor
  ;[1 1 1] When the player is in distance and has enough points, the door will open permanently
  (bind _asfirst_person_character (Utilities|Casting|CastToFirstPersonCharacter (Game|GetPlayerCharacter 0)))
  (if (>= (Variables|/Game/Blueprints/Character/FirstPersonCharacter.FirstPersonCharacter_C|GetPoints _asfirst_person_character) (Variables|Default|GetCost))
    (Utilities|FlowControl|Sequence
      (:then_0
        (bind _asfirst_person_character_2 (Utilities|Casting|CastToFirstPersonCharacter (Game|GetPlayerCharacter 0)))
        (Variables|/Game/Blueprints/Character/FirstPersonCharacter.FirstPersonCharacter_C|SetPoints _asfirst_person_character_2 (- (Variables|/Game/Blueprints/Character/FirstPersonCharacter.FirstPersonCharacter_C|GetPoints _asfirst_person_character_2) (Variables|Default|GetCost))))
      (:then_1
        (Audio|PlaySoundatLocation "/Game/Sounds/DoorOpen.DoorOpen" (Variables|Default|GetBuzzer) "0, 0, 0" 1.0 1.0 0.0 0 0 0))
      (:then_2
        (Audio|PlaySound2D "/Game/Sounds/PurchaseSound.PurchaseSound" 0.5 1.1 0.0 0 0))
      (:then_3
        (bind _sliding (Timeline|Open PlayFromStart)
          (:Update
            (Transformation|SetRelativeLocation (Variables|Default|GetLeftDoor) (Math|Vector|Lerp(Vector) (Variables|Default|GetCurrentLeft) (Variables|Default|GetNewLeft) _sliding) false false)
            (Transformation|SetRelativeLocation (Variables|Default|GetRightDoor) (Math|Vector|Lerp(Vector) (Variables|Default|GetCurrentRight) (Variables|Default|GetNewRight) _sliding) false false))))
      (:then_4
        (Components|DestroyComponent (Variables|Default|GetTrigger))))))

(fn ConstructionScript)