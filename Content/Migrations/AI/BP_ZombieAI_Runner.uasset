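; Runner zombie enemy for a round-based first-person shooter, attacking the player and boarded windows.
; BeginPlay sets the runner flag in the animation Blueprint; capsule hits briefly trigger attacking there.
; Right-hand overlaps damage windows or the player, adding camera shake and knockback, then disable hand collision.
; Damage events reduce health and award points; ZombieDies ragdolls, scores the kill and explodes, while helper functions raise health for rounds.
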(event OnComponentHit(CapsuleComponent)
  (params (HitComponent :type Primitive%20Component%20Object%20Reference) (OtherActor :type Actor%20Object%20Reference) (OtherComp :type Primitive%20Component%20Object%20Reference) (NormalImpulse :type Vector :default "0, 0, 0") (Hit :type Hit%20Result%20Structure%20%28by%20ref%29))
  ;[1 1 1] If the player hits the zombie, the zombie will begin to attack the player
  (Utilities|Casting|CastToFirstPersonCharacter (.hitactor Hit)
    (:then
      (Variables|/Game/AI/Animations/AB_ZombieAI.AB_ZombieAI_C|SetIsAttacking (Variables|Default|GetAs%20AB%20Zombie%20AI) true)
      (Utilities|FlowControl|Delay 1.4)
      (Variables|/Game/AI/Animations/AB_ZombieAI.AB_ZombieAI_C|SetIsAttacking (Variables|Default|GetAs%20AB%20Zombie%20AI) false))
    (:CastFailed
      (bind _asb_window (Utilities|Casting|CastToB_Window (.hitactor Hit)))
      (if (> (Variables|/Game/Blueprints/B_Window.B_Window_C|GetBoardsTotal _asb_window) 0)
        (Variables|/Game/AI/Animations/AB_ZombieAI.AB_ZombieAI_C|SetIsAttacking (Variables|Default|GetAs%20AB%20Zombie%20AI) true)
        (Utilities|FlowControl|Delay 1.4)
        (Variables|/Game/AI/Animations/AB_ZombieAI.AB_ZombieAI_C|SetIsAttacking (Variables|Default|GetAs%20AB%20Zombie%20AI) false)))))

(event OnComponentBeginOverlap(HandRight)
  (params (OverlappedComponent :type Primitive%20Component%20Object%20Reference) (OtherActor :type Actor%20Object%20Reference) (OtherComp :type Primitive%20Component%20Object%20Reference) (OtherBodyIndex :type Integer) (bFromSweep :type Boolean) (SweepResult :type Hit%20Result%20Structure%20%28by%20ref%29))
  ;[1 1 1] When the zombie's hand hits the player, the player will be damaged
  (bind _asfirst_person_character (Utilities|Casting|CastToFirstPersonCharacter OtherActor)
    (:then
      (CallFunction|Attack)
      (Default|PlayerHealing _asfirst_person_character))
    (:CastFailed
      (bind _asb_window (Utilities|Casting|CastToB_Window OtherActor))
      (Default|DamageWindow _asb_window)
      (Collision|SetCollisionEnabled (Variables|Default|GetHandRight) "NoCollision"))))

(event Custom|Ragdoll
  ;[1 1 1] Checks every tick if the zombie's health is above 0, if it isn't then the zombie goes into ragdoll and gives the player points
  (Physics|SetSimulatePhysics (Variables|Character|GetMesh) true)
  (Pawn|Components|CharacterMovement|DisableMovement (Variables|Character|GetCharacterMovement)))

(event Custom|ZombieDies
  (bind _returnvalue (Game|GetPlayerCharacter 0))
  (bind _asfirst_person_character (Utilities|Casting|CastToFirstPersonCharacter _returnvalue))
  ;[1 1 1] Checks every tick if the zombie's health is above 0, if it isn't then the zombie goes into ragdoll and gives the player points
  ;;[1 0 0] When zombie dies, sets the physics to ragdoll, disables the input and gives the player 60 points. After some time the zombie will explode, deleting it from the scene
  (if (<= (Variables|Default|GetHealth) 0.0)
    (CallFunction|Ragdoll)
    (bind _asfirst_person_character_2 (Utilities|Casting|CastToFirstPersonCharacter (Game|GetPlayerCharacter 0)))
    (Variables|/Game/Blueprints/Character/FirstPersonCharacter.FirstPersonCharacter_C|SetPoints _asfirst_person_character_2 (+ (Variables|/Game/Blueprints/Character/FirstPersonCharacter.FirstPersonCharacter_C|GetPoints _asfirst_person_character_2) 60))
    (Components|Activation|SetActive (Variables|Default|GetSoundCue) false false)
    (Collision|SetCollisionEnabled (Variables|Collision|GetCapsuleComponent) "PhysicsOnly")
    (Utilities|FlowControl|Sequence
      (:then_0
        (Audio|PlaySound2D "/Game/Sounds/SC_Bonk.SC_Bonk" 1.7 1.0 0.0 0 0)
        (Math|Integer|IncrementInt (Variables|/Game/Blueprints/Character/FirstPersonCharacter.FirstPersonCharacter_C|GetTotalKills _asfirst_person_character)
          (:%20%20
            (Variables|/Game/Blueprints/Character/FirstPersonCharacter.FirstPersonCharacter_C|SetTotalScore _asfirst_person_character (+ (Variables|/Game/Blueprints/Character/FirstPersonCharacter.FirstPersonCharacter_C|GetTotalScore _asfirst_person_character) 60)))))
      (:then_1
        (Development|PrintString "Zombie is dead")
        (Utilities|FlowControl|Delay 2.0)
        (Effects|SpawnEmitteratLocation "/Game/Particles/P_RocketLauncher_Explosion.P_RocketLauncher_Explosion" (Transformation|GetWorldLocation (Variables|Character|GetMesh)))
        (Audio|PlaySoundatLocation 0 (Variables|/Script/Engine.SceneComponent|GetRelativeLocation (Variables|Character|GetMesh)) "0, 0, 0" 1.0 1.0 0.0 0 0 0)
        (Actor|DestroyActor)))))

(event EventCustomDamageEvent
  (params (DamageAmount :type Float%20%28single-precision%29) (ExtraPoints :type Integer))
  ;[0.8078 0.2902 1] If the player hits this actor with their bullets, this event will be called, reducing the actor's health and add points to the player
  (Variables|Default|SetHealth (- (Variables|Default|GetHealth) DamageAmount))
  (bind _asfirst_person_character (Utilities|Casting|CastToFirstPersonCharacter (Game|GetPlayerCharacter 0)))
  (Variables|/Game/Blueprints/Character/FirstPersonCharacter.FirstPersonCharacter_C|SetPoints _asfirst_person_character (+ (Variables|/Game/Blueprints/Character/FirstPersonCharacter.FirstPersonCharacter_C|GetPoints _asfirst_person_character) ExtraPoints)))

(event EventBeginPlay
  (bind _mesh (Variables|Character|GetMesh))
  ;[1 1 1] Gets the animation instance and sets the zombie to a runner when the game starts, additionally sets hand collision to false
  (bind _asab_zombie_ai (Utilities|Casting|CastToAB_ZombieAI (Components|SkeletalMesh|GetAnimInstance (Variables|Character|GetMesh)))
    (:then
      (Variables|Default|SetAs%20AB%20Zombie%20AI _asab_zombie_ai)
      (Variables|/Game/AI/Animations/AB_ZombieAI.AB_ZombieAI_C|SetIsRunner _asab_zombie_ai true)
      (Collision|SetCollisionEnabled (Variables|Default|GetHandRight) "NoCollision")
      (Utilities|FlowControl|Delay 2.0)
      (bind _returnvalue (Audio|SpawnSoundAttached "/Game/Sounds/ZombieSoundQue.ZombieSoundQue" _mesh "None" (Variables|/Script/Engine.SceneComponent|GetRelativeLocation _mesh) "0, 0, 0" "KeepRelativeOffset" false 0.6 1.0 0.0 "/Game/Sounds/ATT_Zombie.ATT_Zombie" 0))
      (Variables|Default|SetSoundCue _returnvalue))
    (:CastFailed
      (Development|PrintString "Animaton Blueprint wasn't accessed or can't be found"))))

(fn ConstructionScript)

(fn Attack
  (bind _returnvalue (Game|GetPlayerCharacter 0))
  (bind _self self)
  (bind _asfirst_person_character (Utilities|Casting|CastToFirstPersonCharacter _returnvalue))
  (bind _mesh (Variables|Character|GetMesh _self))
  (bind _returnvalue_2 (Math|Vector|GetRightVector _mesh))
  (bind _returnvalue_3 (* _returnvalue_2 1.2e+03))
  ;[1 1 1] The player's health is decreased by a set amount and launches the player slightly back
  (bind _asfirst_person_character_2 (Utilities|Casting|CastToFirstPersonCharacter (Game|GetPlayerCharacter 0)))
  (Default|DepleateHealth _asfirst_person_character_2 (Variables|Default|GetDamage%20Amount))
  (bind _asfirst_person_character_3 (Utilities|Casting|CastToFirstPersonCharacter (Game|GetPlayerCharacter 0)))
  (Camera|PlayWorldCameraShake "/Game/Blueprints/GameFeel/DamageShake.DamageShake_C" (Transformation|GetWorldLocation (Variables|/Game/Blueprints/Character/FirstPersonCharacter.FirstPersonCharacter_C|GetFirstPersonCamera _asfirst_person_character_3)) 0.0 3e+02)
  (Character|LaunchCharacter _asfirst_person_character_3 (Math|Vector|MakeVector (.x _returnvalue_3) (.y _returnvalue_3) 0.0) false false)
  (Collision|SetCollisionEnabled (Variables|Default|GetHandRight) "NoCollision")
  (if (<= (Variables|/Game/Blueprints/Character/FirstPersonCharacter.FirstPersonCharacter_C|GetHealth _asfirst_person_character) 0.0)
    (Variables|/Game/Blueprints/Character/FirstPersonCharacter.FirstPersonCharacter_C|SetIsDead _asfirst_person_character false)
    (Default|PlayerDies _asfirst_person_character)))

(fn LowerRound9Health
  (Variables|Default|SetHealth (+ (Variables|Default|GetHealth) 1e+02)))

(fn HigherRound9Health
  (Variables|Default|SetHealth (* (Variables|Default|GetHealth) 1.1)))