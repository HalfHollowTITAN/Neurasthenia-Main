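; BP_ZombieAI_MainMenu is a zombie character, named as the main menu variant, with melee hit logic.
; BeginPlay clears the runner flag on its animation Blueprint and turns off right-hand collision.
; Capsule hits raise the attacking flag on the stored anim reference for a timed delay.
; Right-hand overlaps call Attack, which depletes player health, launches the player along the mesh's right vector and disables hand collision.
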(event OnComponentHit(CapsuleComponent)
  (params (HitComponent :type Primitive%20Component%20Object%20Reference) (OtherActor :type Actor%20Object%20Reference) (OtherComp :type Primitive%20Component%20Object%20Reference) (NormalImpulse :type Vector :default "0, 0, 0") (Hit :type Hit%20Result%20Structure%20%28by%20ref%29))
  (Utilities|Casting|CastTo (.hitactor Hit))
  (Variables|Default|SetIsAttacking (.As%20AB%20Zombie%20AI (Variables|Default|GetAs%20AB%20Zombie%20AI)) true)
  (Utilities|FlowControl|Delay 1.4)
  (Variables|Default|SetIsAttacking (.As%20AB%20Zombie%20AI (Variables|Default|GetAs%20AB%20Zombie%20AI)) false))

(event OnComponentBeginOverlap(HandRight)
  (params (OverlappedComponent :type Primitive%20Component%20Object%20Reference) (OtherActor :type Actor%20Object%20Reference) (OtherComp :type Primitive%20Component%20Object%20Reference) (OtherBodyIndex :type Integer) (bFromSweep :type Boolean) (SweepResult :type Hit%20Result%20Structure%20%28by%20ref%29))
  (Utilities|Casting|CastTo OtherActor)
  (Utilities|FlowControl|Sequence
    (:then_0
      (CallFunction|Attack))))

(event EventBeginPlay
  (bind _asab_zombie_ai (Utilities|Casting|CastTo (Components|SkeletalMesh|GetAnimInstance (Variables|Character|GetMesh)))
    (:then
      (Variables|Default|SetAs%20AB%20Zombie%20AI 0 _asab_zombie_ai)
      (Variables|Default|SetIsRunner _asab_zombie_ai false)
      (Collision|SetCollisionEnabled (Variables|Default|GetHandRight) "NoCollision"))
    (:CastFailed
      (Development|PrintString "Animaton Blueprint wasn't accessed or can't be found"))))

(fn ConstructionScript)

(fn Attack
  (bind _self self)
  (bind _mesh (Variables|Character|GetMesh _self))
  (bind _returnvalue (Math|Vector|GetRightVector _mesh))
  (bind _returnvalue_2 (* _returnvalue 5e+02))
  (bind _asfirst_person_character (Utilities|Casting|CastTo (Game|GetPlayerCharacter 0)))
  (CallFunction|DepleateHealth _asfirst_person_character (Variables|Default|GetDamage%20Amount))
  (bind _asfirst_person_character_2 (Utilities|Casting|CastTo (Game|GetPlayerCharacter 0)))
  (Character|LaunchCharacter _asfirst_person_character_2 (Math|Vector|MakeVector (.x _returnvalue_2) (.y _returnvalue_2) 0.0) false false)
  (Collision|SetCollisionEnabled (Variables|Default|GetHandRight) "NoCollision"))