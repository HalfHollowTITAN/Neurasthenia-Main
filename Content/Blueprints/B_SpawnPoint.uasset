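; B_SpawnPoint is a spawn point that places zombie AI at its own transform, choosing walker or runner by wave.
; Its construction script copies WaveNumber from an owning B_SpawnManager, while SpawnTarget branches on a separate WaveIdentifier variable.
; Early waves spawn only walkers, middle waves use a random roll favoring walkers over runners, and wave ten onward spawns only runners.
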(fn ConstructionScript
  (bind _asb_spawn_manager (Utilities|Casting|CastToB_SpawnManager (Components|GetOwner)))
  (Variables|Default|SetWave%20Number (Variables|/Game/Blueprints/Managers/B_SpawnManager.B_SpawnManager_C|GetWaveNumber _asb_spawn_manager)))

(fn SpawnTarget
  (bind _returnvalue (Transformation|GetActorTransform))
  (bind _waveidentifier (Variables|Default|GetWaveIdentifier))
  ;[1 1 1] Checks to see if runners can spawn. If its past round 10 only runners will spawn
  (if (<= _waveidentifier 5)
    (Game|SpawnActorfromClass "/Game/AI/BP_ZombieAI_Walker.BP_ZombieAI_Walker_C" (Transformation|GetActorTransform) "Undefined" 0 0)
    (elif (and (>= _waveidentifier 6) (<= _waveidentifier 9))
      (Variables|Default|SetSpawnIdentifier (Math|Random|RandomIntegerinRange 0 20))
      (if (< (Variables|Default|GetSpawnIdentifier) 15)
        (Game|SpawnActorfromClass "/Game/AI/BP_ZombieAI_Walker.BP_ZombieAI_Walker_C" _returnvalue "Undefined" 0 0)
        (else
          (Game|SpawnActorfromClass "/Game/AI/BP_ZombieAI_Runner.BP_ZombieAI_Runner_C" _returnvalue "Undefined" 0 0)))
      (elif (>= _waveidentifier 10)
        (Game|SpawnActorfromClass "/Game/AI/BP_ZombieAI_Runner.BP_ZombieAI_Runner_C" (Transformation|GetActorTransform) "Undefined" 0 0)))))