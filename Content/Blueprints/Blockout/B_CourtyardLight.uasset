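; Blockout courtyard light actor that starts switched off and can be turned on during play.
; BeginPlay hides its two light components and puts the M_light material on its two cylinder meshes.
; The TurnLightsOn event shows both lights and swaps the cylinders to the Light material.
; The file has no path to switch them off again and does not show what calls the event.
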(event Custom|TurnLightsOn
  (Rendering|Material|SetMaterial (Variables|Default|GetCylinder1) 0 "/Game/Materials/Light.Light")
  (Rendering|SetVisibility (Variables|Default|GetLight_1) true false))

(event EventBeginPlay
  (Rendering|Material|SetMaterial (Variables|Default|GetCylinder1) 0 "/Game/Materials/M_light.M_light")
  (Rendering|SetVisibility (Variables|Default|GetLight_1) false false))

(fn ConstructionScript)