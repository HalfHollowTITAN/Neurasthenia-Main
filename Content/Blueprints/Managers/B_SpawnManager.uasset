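; Wave manager that spawns zombies from the spawn points of the player's current room and advances rounds.
; Room overlap volumes select one of five spawner lists, which a fast looping timer feeds into Spawn, paced by a Delay that lengthens after round changes.
; Enemy count grows linearly per wave, with a cap on live enemies.
; When none remain, it increments the wave and spawn-point identifiers, plays a sound and updates the HUD.
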(event OnComponentBeginOverlap(room1)
  (params (OverlappedComponent :type Primitive%20Component%20Object%20Reference) (OtherActor :type Actor%20Object%20Reference) (OtherComp :type Primitive%20Component%20Object%20Reference) (OtherBodyIndex :type Integer) (bFromSweep :type Boolean) (SweepResult :type Hit%20Result%20Structure%20%28by%20ref%29))
  ;[0.1305 0.06354 1] Room Changer(Holds Overlap Events to tell where the player is)
  (Utilities|Casting|CastToFirstPersonCharacter OtherActor)
  (Variables|Default|SetSpawnLocationIdentifier 1))

(event OnComponentBeginOverlap(room3)
  (params (OverlappedComponent :type Primitive%20Component%20Object%20Reference) (OtherActor :type Actor%20Object%20Reference) (OtherComp :type Primitive%20Component%20Object%20Reference) (OtherBodyIndex :type Integer) (bFromSweep :type Boolean) (SweepResult :type Hit%20Result%20Structure%20%28by%20ref%29))
  ;[0.1305 0.06354 1] Room Changer(Holds Overlap Events to tell where the player is)
  (Utilities|Casting|CastToFirstPersonCharacter OtherActor)
  (Variables|Default|SetSpawnLocationIdentifier 3))

(event OnComponentBeginOverlap(room2)
  (params (OverlappedComponent :type Primitive%20Component%20Object%20Reference) (OtherActor :type Actor%20Object%20Reference) (OtherComp :type Primitive%20Component%20Object%20Reference) (OtherBodyIndex :type Integer) (bFromSweep :type Boolean) (SweepResult :type Hit%20Result%20Structure%20%28by%20ref%29))
  ;[0.1305 0.06354 1] Room Changer(Holds Overlap Events to tell where the player is)
  (Utilities|Casting|CastToFirstPersonCharacter OtherActor)
  (Variables|Default|SetSpawnLocationIdentifier 2))

(event OnComponentBeginOverlap(Room4)
  (params (OverlappedComponent :type Primitive%20Component%20Object%20Reference) (OtherActor :type Actor%20Object%20Reference) (OtherComp :type Primitive%20Component%20Object%20Reference) (OtherBodyIndex :type Integer) (bFromSweep :type Boolean) (SweepResult :type Hit%20Result%20Structure%20%28by%20ref%29))
  ;[0.1305 0.06354 1] Room Changer(Holds Overlap Events to tell where the player is)
  (Utilities|Casting|CastToFirstPersonCharacter OtherActor)
  (Variables|Default|SetSpawnLocationIdentifier 4))

(event OnComponentBeginOverlap(Room5)
  (params (OverlappedComponent :type Primitive%20Component%20Object%20Reference) (OtherActor :type Actor%20Object%20Reference) (OtherComp :type Primitive%20Component%20Object%20Reference) (OtherBodyIndex :type Integer) (bFromSweep :type Boolean) (SweepResult :type Hit%20Result%20Structure%20%28by%20ref%29))
  ;[0.1305 0.06354 1] Room Changer(Holds Overlap Events to tell where the player is)
  (Utilities|Casting|CastToFirstPersonCharacter OtherActor)
  (Variables|Default|SetSpawnLocationIdentifier 5))

(event Custom|ActivateSpawner
  (bind _returnvalue (Game|GetPlayerCharacter 0))
  (bind _spawnerlist4 (Variables|Default|GetSpawnerList4))
  (bind _spawnerlist5 (Variables|Default|GetSpawnerList5))
  (bind _spawnerlist1 (Variables|Default|GetSpawnerList1))
  (bind _spawnerlist2 (Variables|Default|GetSpawnerList2))
  (bind _spawnerlist3 (Variables|Default|GetSpawnerList3))
  ;[1 1 1] Spawns zombire based on the active round. Sets the active spawn zone based on room number that is active
  (if (and (> (Variables|Default|GetEneimeAmount) 0) (<= (Variables|Default|GetEneimesRemaining) 49))
    ;;[1 0 0.3634] Spawn Location Manager(Enables Appropriate Spawners for the corresponding room)
    (switch int (Variables|Default|GetSpawnLocationIdentifier)
      (:1
        (Utilities|Spawn _spawnerlist1 _spawnerlist1
          (:Exec
            (Variables|Default|SetSwapping false))))
      (:2
        (Utilities|Spawn _spawnerlist2 _spawnerlist2
          (:Exec
            (Variables|Default|SetSwapping false))))
      (:3
        (Utilities|Spawn _spawnerlist3 _spawnerlist3
          (:Exec
            (Variables|Default|SetSwapping false))))
      (:4
        (Utilities|Spawn _spawnerlist4 _spawnerlist4
          (:Exec
            (Variables|Default|SetSwapping false))))
      (:5
        (Utilities|Spawn _spawnerlist5 _spawnerlist5
          (:Exec
            (Variables|Default|SetSwapping false)))))
    (else
      ;;[1 0.07523 0] Starts new round when all enemies are dead
      (bind _outactors (Actor|GetAllActorswithInterface "/Game/Blueprints/Blueprint_Interfaces/BPI_Eneimes.BPI_Eneimes_C"))
      (bind _output_get (Variables|Default|SetSpawnArray _outactors))
      (Variables|Default|SetEneimesRemaining (Utilities|Array|Length _output_get))
      (if (<= (Variables|Default|GetEneimesRemaining) 0)
        (Math|Integer|IncrementInt (Variables|Default|GetWaveNumber)
          (:%20%20
            (if true
              (CallFunction|EnemyCalculation)
              (Utilities|FlowControl|Sequence
                (:then_0
                  (Audio|PlaySound2D "/Game/Sounds/WaveChange.WaveChange" 1.0 1.0 0.0 0 0)
                  (Variables|Default|SetSwapping true)
                  (bind _outactors_2 (Actor|GetAllActorsOfClass "/Game/Blueprints/B_SpawnPoint.B_SpawnPoint_C"))
                  (for _array_element _outactors_2
                    (Math|Integer|IncrementInt (Variables|/Game/Blueprints/B_SpawnPoint.B_SpawnPoint_C|GetWaveIdentifier _array_element))))
                (:then_1
                  (if (Variables|Default|GetSwapping)
                    (bind _asfirst_person_character (Utilities|Casting|CastToFirstPersonCharacter _returnvalue))
                    (Default|ChangeRoundAnimation (Variables|/Game/Blueprints/Character/FirstPersonCharacter.FirstPersonCharacter_C|GetHUD _asfirst_person_character))))
                (:then_2
                  (bind _asfirst_person_character_2 (Utilities|Casting|CastToFirstPersonCharacter _returnvalue))
                  (Default|UpdateNumberedRound (Variables|/Game/Blueprints/Character/FirstPersonCharacter.FirstPersonCharacter_C|GetHUD _asfirst_person_character_2))
                  (Math|Integer|IncrementInt (Variables|/Game/Blueprints/Character/FirstPersonCharacter.FirstPersonCharacter_C|GetHighestWave _asfirst_person_character_2)))))))))))

(event EventBeginPlay
  ;[1 1 1] Spawns zombire based on the active round. Sets the active spawn zone based on room number that is active
  (Math|Integer|IncrementInt (Variables|Default|GetWaveNumber)
    (:%20%20
      (CallFunction|EnemyCalculation)
      (Variables|Default|SetSpawnLocationIdentifier 1)
      (Variables|Default|SetZombieNewHealth 1e+02)
      (Utilities|Time|SetTimerbyEvent (delegate Custom|ActivateSpawner) 0.1 true))))

(fn ConstructionScript)

(fn EnemyCalculation
  (Variables|Default|SetEneimeAmount (- (* (Variables|Default|GetWaveNumber) 5) (* (Variables|Default|GetWaveNumber) 2))))

(fn EnemyHealthCalc
  (if (<= (Variables|Default|GetWaveIdentifier) 9)
    (Variables|Default|SetZombieNewHealth (+ (Variables|Default|GetZombieNewHealth) 4e+01))
    (else
      (Variables|Default|SetZombieNewHealth (* (Variables|Default|GetZombieNewHealth) 1.1)))))