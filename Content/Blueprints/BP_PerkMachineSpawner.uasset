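; Perk machine spawner that places random perk machine classes at arrow markers on BeginPlay.
; A loop spawns from ActorClass at LocationUsed, then picks the next random SpawnList arrow, removing the used class and new arrow to limit repeats.
; LocationUsed updates after each spawn, and the construction script lists Perk4Arrow twice.
; An older MachineID rotation shuffle is disconnected and never runs.
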(event EventBeginPlay
  (for _index (range 0 3)
    (if true
      (bind _returnvalue (Game|SpawnActorfromClass (.OutItem (Utilities|Array|Random (Variables|Default|GetActor%20Class))) (Math|Transform|MakeTransform (Transformation|GetWorldLocation (Variables|Default|GetLocationUsed)) (Transformation|GetWorldRotation (Variables|Default|GetLocationUsed)) "0.800000,0.800000,0.800000") "Undefined" 0 0))
      (bind _output_get (Variables|Default|SetLocationUsed (.OutItem (Utilities|Array|Random (Variables|Default|GetSpawnList)))))
      (bind _returnvalue_2 (Utilities|Array|RemoveItem (Variables|Default|GetActor%20Class) (Utilities|GetClass _returnvalue)))
      (Development|PrintString (Utilities|String|ToString(Boolean) _returnvalue_2))
      (bind _returnvalue_3 (Utilities|Array|RemoveItem (Variables|Default|GetSpawnList) _output_get))
      (Development|PrintString (Utilities|String|ToString(Boolean) _returnvalue_3))
      (Development|PrintString (Utilities|GetDisplayName _output_get) true true "(R=0.000000,G=0.660000,B=1.000000,A=1.000000)" 1e+01)))
  (Development|PrintString "Complete"))

(event Collision|EventActorBeginOverlap
  (params (OtherActor :type Actor%20Object%20Reference)))

(fn ConstructionScript
  (bind _perk4_arrow (Variables|Default|GetPerk4%20Arrow))
  (Variables|Default|SetSpawnList (Utilities|Array|MakeArray (Variables|Default|GetPerk1%20Arrow) (Variables|Default|GetPerk2%20Arrow) (Variables|Default|GetPerk3%20Arrow) _perk4_arrow _perk4_arrow)))