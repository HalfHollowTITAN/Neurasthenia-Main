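; Barricade window with six boards that can be knocked off by damage and repaired by the player for points.
; DamageWindow and RepairWindow step BoardsTotal between zero and six, toggling the matching board's visibility and collision.
; Each repair plays a purchase sound and adds to the player's points and total score.
; TextTrigger overlaps show or hide the HUD repair prompt, which also hides once the window is fully boarded.
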(event OnComponentBeginOverlap(TextTrigger)
  (params (OverlappedComponent :type Primitive%20Component%20Object%20Reference) (OtherActor :type Actor%20Object%20Reference) (OtherComp :type Primitive%20Component%20Object%20Reference) (OtherBodyIndex :type Integer) (bFromSweep :type Boolean) (SweepResult :type Hit%20Result%20Structure%20%28by%20ref%29))
  (if (< (Variables|Default|GetBoardsTotal) 6)
    (bind _asfirst_person_character (Utilities|Casting|CastToFirstPersonCharacter OtherActor))
    (Default|ChangeKeyText(Repair) (Variables|/Game/Blueprints/Character/FirstPersonCharacter.FirstPersonCharacter_C|GetHUD _asfirst_person_character))))

(event OnComponentEndOverlap(TextTrigger)
  (params (OverlappedComponent :type Primitive%20Component%20Object%20Reference) (OtherActor :type Actor%20Object%20Reference) (OtherComp :type Primitive%20Component%20Object%20Reference) (OtherBodyIndex :type Integer))
  (bind _asfirst_person_character (Utilities|Casting|CastToFirstPersonCharacter OtherActor))
  (Default|HideText (Variables|/Game/Blueprints/Character/FirstPersonCharacter.FirstPersonCharacter_C|GetHUD _asfirst_person_character)))

(fn ConstructionScript
  (Utilities|FlowControl|Sequence))

(fn DamageWindow
  (bind (_board_6 _board_5 _board_4 _board_3 _board_2 _board_1) (Utilities|BoardsOutputs))
  ;[0 1 0.2166] Check to see if there are more than 0 boards. If there then the boards will be decreased by one per hit. Hits will never proceed past 0
  (if (> (Variables|Default|GetBoardsTotal) 0)
    (Variables|Default|SetBoardsTotal (- (Variables|Default|GetBoardsTotal) 1))
    ;[1 0.8339 0] Disables boards based on the int switch. Each board is disabled seperately
    (switch int (Variables|Default|GetBoardsTotal)
      (:0
        (Rendering|SetVisibility _board_1 false false)
        (Collision|SetCollisionEnabled (Variables|Default|GetBoard_1) "NoCollision"))
      (:1
        (Rendering|SetVisibility _board_2 false false)
        (Collision|SetCollisionEnabled (Variables|Default|GetBoard_2) "NoCollision"))
      (:2
        (Rendering|SetVisibility _board_3 false false)
        (Collision|SetCollisionEnabled (Variables|Default|GetBoard_3) "NoCollision"))
      (:3
        (Rendering|SetVisibility _board_4 false false)
        (Collision|SetCollisionEnabled (Variables|Default|GetBoard_4) "NoCollision"))
      (:4
        (Rendering|SetVisibility _board_5 false false)
        (Collision|SetCollisionEnabled (Variables|Default|GetBoard_5) "NoCollision"))
      (:5
        (Rendering|SetVisibility _board_6 false false)
        (Collision|SetCollisionEnabled (Variables|Default|GetBoard_6) "NoCollision")))))

(fn RepairWindow
  (bind (_board_6 _board_5 _board_4 _board_3 _board_2 _board_1) (Utilities|BoardsOutputs))
  ;[1 1 1] Checks if there are less than 6 boards. If there is then the boards value will increase by one per call and will clap between 0 and 6
  (if (< (Variables|Default|GetBoardsTotal) 6)
    (Variables|Default|SetBoardsTotal (Math|Integer|Clamp(Integer) (+ (Variables|Default|GetBoardsTotal) 1) 0 6))
    (switch int (Variables|Default|GetBoardsTotal)
      (:1
        ;[1 0.9305 0] Board visibility is re-enabled based on the int switch
        ;;[1 1 1] Board 1
        (Rendering|SetVisibility _board_1 true false)
        (Collision|SetCollisionEnabled (Variables|Default|GetBoard_1) "QueryOnly"))
      (:2
        ;;[1 1 1] Board 2
        (Rendering|SetVisibility _board_2 true false)
        (Collision|SetCollisionEnabled (Variables|Default|GetBoard_2) "QueryOnly"))
      (:3
        ;;[1 1 1] Board 3
        (Rendering|SetVisibility _board_3 true false)
        (Collision|SetCollisionEnabled (Variables|Default|GetBoard_3) "QueryOnly"))
      (:4
        ;;[1 1 1] Board 4
        (Rendering|SetVisibility _board_4 true false)
        (Collision|SetCollisionEnabled (Variables|Default|GetBoard_4) "QueryOnly"))
      (:5
        ;;[1 1 1] Board 5
        (Rendering|SetVisibility _board_5 true false)
        (Collision|SetCollisionEnabled (Variables|Default|GetBoard_5) "QueryOnly"))
      (:6
        ;;[1 1 1] Board 6
        (Rendering|SetVisibility _board_6 true false)
        (Collision|SetCollisionEnabled (Variables|Default|GetBoard_6) "QueryOnly")))
    ;[1 0.3426 0] When a board is added, the player will have 10 points added to both their points and their overall score and the interaction text will be hidden
    (Audio|PlaySound2D "/Game/Sounds/PurchaseSound.PurchaseSound" 1.0 1.0 0.0 0 0)
    (bind _asfirst_person_character (Utilities|Casting|CastToFirstPersonCharacter (Game|GetPlayerCharacter 0)))
    (Variables|/Game/Blueprints/Character/FirstPersonCharacter.FirstPersonCharacter_C|SetPoints _asfirst_person_character (+ (Variables|/Game/Blueprints/Character/FirstPersonCharacter.FirstPersonCharacter_C|GetPoints _asfirst_person_character) 10))
    (Variables|/Game/Blueprints/Character/FirstPersonCharacter.FirstPersonCharacter_C|SetTotalScore _asfirst_person_character (+ (Variables|/Game/Blueprints/Character/FirstPersonCharacter.FirstPersonCharacter_C|GetTotalScore _asfirst_person_character) 10))
    (if (== (Variables|Default|GetBoardsTotal) 6)
      (Default|HideText (Variables|/Game/Blueprints/Character/FirstPersonCharacter.FirstPersonCharacter_C|GetHUD (.AsFirst%20Person%20Character (Utilities|Casting|CastToFirstPersonCharacter (Game|GetPlayerCharacter 0))))))))