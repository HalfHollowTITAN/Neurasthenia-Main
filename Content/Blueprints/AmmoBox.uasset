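; AmmoBox is a purchasable ammo refill point that restores the player's total ammo in exchange for points.
; Its TextTrigger overlap shows an "E" buy prompt with the cost on the FirstPersonCharacter's HUD and hides it on exit.
; RefillAmmo, not called within this file, checks that player 0 can afford it and is below TotalAmmoDefault, then refills, deducts Cost and plays reload and purchase sounds.
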(event OnComponentBeginOverlap(TextTrigger)
  (params (OverlappedComponent :type Primitive%20Component%20Object%20Reference) (OtherActor :type Actor%20Object%20Reference) (OtherComp :type Primitive%20Component%20Object%20Reference) (OtherBodyIndex :type Integer) (bFromSweep :type Boolean) (SweepResult :type Hit%20Result%20Structure%20%28by%20ref%29))
  (bind _asfirst_person_character (Utilities|Casting|CastToFirstPersonCharacter OtherActor))
  (Default|ChangeKeyText(AmmoBuy) (Variables|/Game/Blueprints/Character/FirstPersonCharacter.FirstPersonCharacter_C|GetHUD _asfirst_person_character) "E" (Utilities|Text|ToText(Integer) (Variables|Default|GetCost))))

(event OnComponentEndOverlap(TextTrigger)
  (params (OverlappedComponent :type Primitive%20Component%20Object%20Reference) (OtherActor :type Actor%20Object%20Reference) (OtherComp :type Primitive%20Component%20Object%20Reference) (OtherBodyIndex :type Integer))
  (bind _asfirst_person_character (Utilities|Casting|CastToFirstPersonCharacter OtherActor))
  (Default|HideText (Variables|/Game/Blueprints/Character/FirstPersonCharacter.FirstPersonCharacter_C|GetHUD _asfirst_person_character)))

(event EventBeginPlay)

(fn ConstructionScript)

(fn RefillAmmo
  (bind _returnvalue (Game|GetPlayerCharacter 0))
  (bind _asfirst_person_character (Utilities|Casting|CastToFirstPersonCharacter _returnvalue))
  (bind _totalammodefault (Variables|/Game/Blueprints/Character/FirstPersonCharacter.FirstPersonCharacter_C|GetTotalAmmoDefault _asfirst_person_character))
  ;[1 1 1] Checks if the player has enough points. If they do then their total ammo is restored to its max using the Total ammo default anf the cost is deducted from the player's points
  (if (and (>= (Variables|/Game/Blueprints/Character/FirstPersonCharacter.FirstPersonCharacter_C|GetPoints _asfirst_person_character) (Variables|Default|GetCost)) (< (Variables|/Game/Blueprints/Character/FirstPersonCharacter.FirstPersonCharacter_C|GetTotalAmmo _asfirst_person_character) _totalammodefault))
    (Variables|/Game/Blueprints/Character/FirstPersonCharacter.FirstPersonCharacter_C|SetTotalAmmo _asfirst_person_character _totalammodefault)
    (Variables|/Game/Blueprints/Character/FirstPersonCharacter.FirstPersonCharacter_C|SetPoints _asfirst_person_character (- (Variables|/Game/Blueprints/Character/FirstPersonCharacter.FirstPersonCharacter_C|GetPoints _asfirst_person_character) (Variables|Default|GetCost)))
    (Audio|PlaySound2D "/Game/PrototypeWeap/Sound/Rifle/Rifle_Reload05.Rifle_Reload05" 1.0 1.0 0.0 0 0)
    (Audio|PlaySound2D "/Game/Sounds/PurchaseSound.PurchaseSound" 1.0 1.0 0.0 0 0)))