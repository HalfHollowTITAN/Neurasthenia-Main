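; Meteor stand interactable for a hidden Easter egg song, playing a quiet attenuated idle sound at its location from level start.
; Interacting decrements a shared InteractsLeft counter on the FirstPersonCharacter, plays a feedback sound and sets the trigger to ignore Visibility and Camera traces.
; When the counter reaches zero, the song plays in 2D after a short delay.
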(event Custom|Interact
  (bind _returnvalue (Game|GetPlayerCharacter 0))
  (bind _interacttrigger (Variables|Default|GetInteractTrigger))
  (bind _asfirst_person_character (Utilities|Casting|CastToFirstPersonCharacter _returnvalue))
  (bind _interactsleft (Variables|/Game/Blueprints/Character/FirstPersonCharacter.FirstPersonCharacter_C|GetInteractsLeft _asfirst_person_character))
  ;[1 1 1] Will cause an interaction event. If the player interacts with three meteor stands then the Easter Egg song will play.
  (if (not (<= _interactsleft 0))
    (Math|Integer|DecrementInt _interactsleft
      (:%20%20
        (Audio|PlaySoundatLocation "/Game/Sounds/EE_Interaction.EE_Interaction" (Transformation|GetWorldLocation (Variables|Default|GetSoundLocations)) "0, 0, 0" 1.5 5.0 0.0 0 0 0 0)
        (Collision|SetCollisionResponsetoChannel _interacttrigger "ECC_Visibility" "ECR_Ignore")
        (Collision|SetCollisionResponsetoChannel _interacttrigger "ECC_Camera" "ECR_Ignore")
        (if (<= _interactsleft 0)
          (Utilities|FlowControl|Delay 2.0)
          (CallFunction|PlaySound))))))

(event EventBeginPlay
  ;[1 1 1] Begins playing ambient sound when level starts
  (Audio|PlaySoundatLocation "/Game/Sounds/Meteor_Idle.Meteor_Idle" (Transformation|GetWorldLocation (Variables|Default|GetSoundLocations)) "0, 0, 0" 0.1 1.0 0.0 "/Game/Sounds/MeteorAtt.MeteorAtt" 0 0 0))

(fn ConstructionScript)

(fn PlaySound
  (Audio|PlaySound2D "/Game/Sounds/EasterEggSong.EasterEggSong" 1.0 1.0 0.0 0 0))